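; Game state Blueprint that tracks the match time limit and announces when the match is over.
; On BeginPlay, the server starts a looping timer and copies the maximum match duration from the Juego_Brinco game mode.
; Each timer tick compares ElapsedTime to that limit and, once it is reached, only prints an end-of-match message, repeating because the timer is never cleared.
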(event `self.ReceiveBeginPlay`
  ;[1 1 1] Tiempo Restante Juego
  (`/Engine/EditorBlueprintResources/ActorMacros.Switch Has Authority`
    (:`Authority`
      (`KismetSystemLibrary.K2_SetTimerDelegate` (delegate `TiempoPartida`) 0.5 true)
      (bind _asjuego_brinco (cast `/Game/Mi_Carpeta/GameMode/Juego_Brinco` (`GameplayStatics.GetGameMode`)))
      (set `self.TiempoMaximo` (`/Game/Mi_Carpeta/GameMode/Juego_Brinco.TiempoMaximoPartida` _asjuego_brinco)))))

(event `TiempoPartida`
  ;[1 1 1] Tiempo Restante Juego
  (if (>= (`self.ElapsedTime`) (`self.TiempoMaximo`))
    (`KismetSystemLibrary.PrintString` "La partida termino")))

(fn `UserConstructionScript`)